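; Game instance for a FNAF game, declaring the global interface for save data, level flow and progression.
; Its functions cover coins, prizes, glitches, achievements, Glitchtrap stages, nightmare mode, fade-outs and loading of menus, hubs and levels.
; Nearly all are empty stubs or return defaults.
; Only subtitle query, a toggle that always disables subtitles, and LoadLevel, which opens a level by name from level info, have logic.
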(fn GetSubtitleson
  (return (Class|GameplayStatics|AreSubtitlesEnabled)))

(fn GiveAllAchievements)

(fn GetAvailablePrizesforLevel
  (return 0))

(fn AttemptAwardSpecialPrize)

(fn SaveGameSlot)

(fn CheckforAchievementCompletion)

(fn GiveBasketBall
  (params (Prize :type Prize%20Item%20Struct%20Structure)))

(fn HasDefeatedGlitchtrap
  (params (GlitchtrapDefeated :type Boolean)))

(fn DefeatGlitchtrap)

(fn SetGlitchListenedto
  (params (NewItem :type Integer)))

(fn GetInstructionWidget
  (return 0))

(fn UnlockAllPrizes)

(fn UnlockAllGlitches)

(fn GetAchievementData
  (return "None" 0.0 0.0 "" "" false))

(fn FadeOutwithLevelLoad
  (params (LevelToLoadAfterFade :type Name) (Skip_Fade_out :type Boolean) (ShowLoadingScreen :type Boolean)))

(fn AwardGlitch
  (params (GlitchID :type Integer)))

(fn HasGlitch
  (params (GlitchID :type Integer) (Value :type Boolean)))

(fn UpdateGlitchtrapStage)

(fn GetGlitchtrapStage
  (return 0))

(fn InitSaveGame)

(fn HasCoin
  (params (CoinID :type Integer)))

(fn GetSavedLevelInfo
  (return ""))

(fn HasPrize
  (params (PrizeID :type Name) (HasPrize :type Boolean)))

(fn EnableNightmareMode
  (params (IsInNightmareMode :type Boolean)))

(fn IsNightmareModeEnabled
  (return false))

(fn GetLevelNumber
  (return 0))

(fn AwardRandomPrize
  (params (ValidPrize :type Boolean) (Prize :type Prize%20Item%20Struct%20Structure) (PrizeID :type Name)))

(fn GetRandomAvailablePrize
  (return false "" ""))

(fn GetAvailablePrizesBase
  (return 0))

(fn GetNumberOfPlayers
  (return 0))

(fn GetAllLevelsOfType
  (return "NewEnumerator0" 0 0))

(fn IsLevelUnlocked
  (return "None" false))

(fn IsLevelBeaten
  (return "None" false))

(fn IsShowtimeUnlocked
  (return false))

(fn FindCurrentLevelID)

(fn UpdateCachedCoinCount)

(fn ClearSaveGame)

(fn GetCurrentLevelID
  (return "None"))

(fn GetCurrentLevelInfo
  (return "" 0))

(fn UnlockCoin
  (params (CoinID :type Integer)))

(fn GetSaveGame
  (return 0))

(fn SaveLevelVictory)

(fn SetupPlayerCharacters
  (params (LobbyPlayers :type Array%20of%20Lobby%20Player%20Controller%20Object%20References)))

(fn GetCoinCount
  (return 0))

(fn GetLevelInstructions
  (return "" false))

(fn SpawnLevelDatabase)

(fn LoadMainMenu)

(fn UnlockAllLevels)

(fn RunFadeOut)

(fn LoadTitle)

(fn LoadIntroLevel)

(fn LoadGlichedIntroLevel)

(fn LoadGallery)

(fn FinaleVictory
  (params (NumCoins :type Integer)))

(fn UnlockAllCoins)

(fn ToggleSubtitles
  (Class|GameplayStatics|SetSubtitlesEnabled false))

(fn LoadGlitchKeyhole)

(fn LoadCasetteRoom)

(fn LoadGameOver)

(fn LevelVictory
  (params (NumCoins :type Integer) (No_Fade_Out_at_end :type Boolean)))

(fn LoadHalloweenHub)

(fn ForceLoadHTitle)

(fn LoadMainHub)

(fn LevelDefeat)

(fn RestartCurrentLevel)

(fn LoadHSplash)

(fn LoadGearGame)

(fn LoadDarkRide)

(fn FinishCaveat
  (params (Difficulty :type Integer)))

(fn LoadHollidayLevel)

(fn LoadLevel
  (params (LevelID :type Name) (LevelInfo :type Level%20Info%20Struct%20Structure))
  (Game|OpenLevel(byName) (Utilities|String|StringToName (.leveltoload LevelInfo))))