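; PrintTest_BP is a test tool Blueprint that briefly displays a message through a text render component when play begins.
; On BeginPlay it makes the TextRender visible and sets its text from the PrintString variable.
; After a delay set by DelayClearTime, it hides the text again, and the construction script is empty.
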(event EventBeginPlay
  (bind _textrender (Variables|Default|GetTextRender))
  (Rendering|SetVisibility _textrender true false)
  (Rendering|Components|TextRender|SetText _textrender (Utilities|Text|ToText(String) (Utilities|String|ToString(Text) (Utilities|Text|ToText(String) (Variables|Default|GetPrint_String)))))
  (Utilities|FlowControl|Delay (Variables|Default|GetDelay%20Clear%20time))
  (Rendering|SetVisibility (Variables|Default|GetTextRender) false false))

(event Input|KeyboardEvents|ObjectPath:Freddys/Content/ProductionAssets/Data/Level/GameTypeMapper.2
  (params (Key :type Key%20Structure)))

(fn ConstructionScript)