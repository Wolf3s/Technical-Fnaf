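; BP_FNAFGameMode is a game mode Blueprint for an FNAF game that holds mostly debug or test logic, with no gameplay rules.
; The Widget event displays a Test widget.
; The Voxxid event reports the GPU brand, first forcing extreme screen percentage and Epic scalability on Intel GPUs.
; An unconnected chain would unlock the console, install a cheat manager and enable subtitles, but it never runs.
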(event Custom|Widget
  (bind _returnvalue (UserInterface|CreateWidget "/Game/ProductionAssets/Blueprints/BackEnd/Widgets/Test.Test_C"))
  (UserInterface|Viewport|AddtoViewport _returnvalue 0))

(event Custom|Voxxid
  (bind _returnvalue (Class|FNAFGameInstanceBase|GetPrimaryGPUBrand))
  (if (Utilities|String|StartsWith (Class|FNAFGameInstanceBase|GetPrimaryGPUBrand) "INTEL")
    (Development|ExecuteConsoleCommand "r.screenpercentage 500" 0)
    (Class|AutomationBlueprintFunctionLibrary|SetScalabilityQualitytoEpic)
    (Class|GameMode|Say _returnvalue)
    (else
      (Class|GameMode|Say _returnvalue))))

(event Custom|ucc)

(event EventBeginPlay
  (|CallParentFunction))

(event EventTick
  (params (DeltaSeconds :type Float%20%28single-precision%29))
  (|CallParentFunction DeltaSeconds) ; This node is disabled and will not be called.\nDrag off pins to build functionality.
)

(fn ConstructionScript
  (|CallParentFunction))